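; UDP connection Blueprint for a Ukaton Mission device, carrying bytes between the game and a given IP address.
; Connect opens the send socket, whose opened event then opens a receive socket on an available port and starts a looping one-second ping timer.
; Received bytes go to ParseMessage, while EmitBytes forwards outgoing data.
; Disconnect, also called on EndPlay, runs DisconnectImplementation, closes the send socket and clears the timer.
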(event `self.Connect`
  (params (IPAddress :type String))
  (`UDPComponent.OpenSendSocket` (`self.UDP`) IPAddress (`self.GetSendPort`)))

(event `self.ReceiveEndPlay`
  (params (EndPlayReason :type "EEndPlayReason Enum" :default "Destroyed"))
  (`self.Disconnect`))

(event `self.UDP.OnSendSocketOpened`
  (params (SpecifiedPort :type Integer) (BoundPort :type Integer) (BoundIP :type String))
  (bind _outport (`UDPPortUtils.FindAvailableUdpPort`))
  (bind _returnvalue (`self.SetInListenPort` _outport))
  (`UDPComponent.OpenReceiveSocket` (`self.UDP`) "0.0.0.0" _returnvalue)
  (bind _returnvalue_2 (`KismetSystemLibrary.K2_SetTimer` null "Ping" 1.0 true)))

(event `self.UDP.OnReceiveSocketOpened`
  (params (Port :type Integer))
  (`KismetSystemLibrary.PrintString` (`KismetStringLibrary.Conv_IntToString` Port) true false (struct :`G` 0.66 :`B` 1.0 :`A` 1.0) 10.0))

(event `self.Disconnect`
  (`KismetSystemLibrary.PrintString` "disconnecting")
  (`self.Disconnect_Implementation`)
  (`UDPComponent.CloseSendSocket` (`self.UDP`))
  (`KismetSystemLibrary.K2_ClearAndInvalidateTimerHandle` (stale `self.UDP.OnSendSocketOpened` _returnvalue_2)))

(event `self.UDP.OnReceivedBytes`
  (params (Bytes :type "Array of Byte (by ref)") (IPAddress :type String) (Port :type "Integer (by ref)"))
  (`KismetSystemLibrary.PrintString` "received bytes" false false)
  (`self.ParseMessage` Bytes))

(event `self.EmitBytes`
  (params (Data :type "Array of Byte (by ref)"))
  (`UDPComponent.EmitBytes` (`self.UDP`) Data))

(fn `Ping`
  (`UDPComponent.EmitBytes` (`self.UDP`) (`self.GetPingMessage`))
  (`KismetSystemLibrary.PrintString` "PING" false)
  (return))

(fn `UserConstructionScript`)