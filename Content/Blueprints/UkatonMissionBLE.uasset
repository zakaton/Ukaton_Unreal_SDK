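; UkatonMissionBLE is an early-stage Blueprint for Bluetooth Low Energy communication, presumably with Ukaton Mission devices.
; On BeginPlay it creates and stores a BLE manager, checks platform support and requests that Bluetooth turn on.
; After a short delay it prints whether Bluetooth is enabled, or reports immediately if BLE is unsupported.
; Connect and Disconnect events are empty stubs, and the service-UUID-filtered device scan is not wired to run.
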(event `self.ReceiveBeginPlay`
  (bind _returnvalue (`BleUtils.CreateBleManager`))
  (bind _output_get (set `self.BleManager` _returnvalue))
  (if (`BleManagerInterface.IsBleSupported` _output_get)
    (`BleManagerInterface.SetBluetoothState` (`self.BleManager`) true)
    (`KismetSystemLibrary.Delay` 0.5)
    (if (`BleManagerInterface.IsBluetoothEnabled` (`self.BleManager`))
      (`KismetSystemLibrary.PrintString` "ENABLED")
      (else
        (`KismetSystemLibrary.PrintString` "DISABLED")))
    (else
      (`KismetSystemLibrary.PrintString` "BLE NOT SUPPORTED"))))

(event `self.Connect`
  (params (Name :type String)))

(event `self.Disconnect`)

(fn `UserConstructionScript`)