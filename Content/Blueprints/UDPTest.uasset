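; A test actor for two-way UDP messaging through a UDP component, printing debug text on screen.
; On BeginPlay it opens a send socket to a hard-coded LAN address, then opens a receive socket on the same bound port and starts a looping timer that emits a ping each second.
; Received bytes only print a notice; a separate GetInfo function sends an info request.
; EndPlay closes the send socket and clears the timer.
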(event `self.ReceiveBeginPlay`
  (`UDPComponent.OpenSendSocket` (`self.UDP`) "192.168.1.30" 9999))

(event `self.ReceiveEndPlay`
  (params (EndPlayReason :type "EEndPlayReason Enum" :default "Destroyed"))
  (`UDPComponent.CloseSendSocket` (`self.UDP`))
  (`KismetSystemLibrary.K2_ClearAndInvalidateTimerHandle` (stale `self.UDP.OnSendSocketOpened` _returnvalue)))

(event `self.UDP.OnSendSocketOpened`
  (params (SpecifiedPort :type Integer) (BoundPort :type Integer) (BoundIP :type String))
  (`UDPComponent.OpenReceiveSocket` (`self.UDP`) "0.0.0.0" BoundPort)
  (bind _returnvalue (`KismetSystemLibrary.K2_SetTimer` null "Ping" 1.0 true)))

(event `self.UDP.OnReceiveSocketOpened`
  (params (Port :type Integer))
  (`KismetSystemLibrary.PrintString` (`KismetStringLibrary.Conv_IntToString` Port) true true (struct :`G` 0.66 :`B` 1.0 :`A` 1.0) 10.0))

(event `self.UDP.OnReceivedBytes`
  (params (Bytes :type "Array of Byte (by ref)") (IPAddress :type String) (Port :type "Integer (by ref)"))
  (`KismetSystemLibrary.PrintString` "received bytes" true true (struct :`R` 0.292796 :`G` 1.0 :`B` 0.221533 :`A` 1.0) 10.0))

(fn `getInfo`
  (`UDPComponent.EmitBytes` (`self.UDP`) (`self.getInfoArray`))
  (`KismetSystemLibrary.PrintString` "Requested Info")
  (return))

(fn `ping`
  (`UDPComponent.EmitBytes` (`self.UDP`) (`self.pingMessage`))
  (`KismetSystemLibrary.PrintString` "Ping!" true true (struct :`G` 0.66 :`B` 1.0 :`A` 1.0) 1.0)
  (return))

(fn `UserConstructionScript`)