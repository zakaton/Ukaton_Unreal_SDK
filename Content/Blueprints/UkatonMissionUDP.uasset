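; Blueprint that manages a UDP connection to an Ukaton Mission device.
; Connect opens a send socket to the given IP, then its callback opens a receive socket on a free local port and starts a looping one-second Ping timer.
; Received bytes go to ParseMessage, and GetInfo sends an info request.
; Disconnect, also run on EndPlay, closes the send socket, clears the timer and resets the handshake flags.
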(event `self.Connect`
  (params (IPAddress :type String))
  (`UDPComponent.OpenSendSocket` (`self.UDP`) IPAddress (`self.GetSendPort`)))

(event `self.ReceiveEndPlay`
  (params (EndPlayReason :type "EEndPlayReason Enum" :default "Destroyed"))
  (`self.Disconnect`))

(event `self.UDP.OnSendSocketOpened`
  (params (SpecifiedPort :type Integer) (BoundPort :type Integer) (BoundIP :type String))
  (bind _outport (`UDPPortUtils.FindAvailableUdpPort`))
  (bind _output_get (set `self.InListenPort` _outport))
  (`UDPComponent.OpenReceiveSocket` (`self.UDP`) "0.0.0.0" _output_get)
  (bind _returnvalue (`KismetSystemLibrary.K2_SetTimer` null "Ping" 1.0 true)))

(event `self.UDP.OnReceiveSocketOpened`
  (params (Port :type Integer))
  (`KismetSystemLibrary.PrintString` (`KismetStringLibrary.Conv_IntToString` Port) true true (struct :`G` 0.66 :`B` 1.0 :`A` 1.0) 10.0))

(event `self.Disconnect`
  (`UDPComponent.CloseSendSocket` (`self.UDP`))
  (`KismetSystemLibrary.K2_ClearAndInvalidateTimerHandle` (stale `self.UDP.OnSendSocketOpened` _returnvalue))
  (set `self.bDidSendSetInListenPortMessage` false)
  (set `self.bDidReceiveDeviceInfo` false))

(event `self.UDP.OnReceivedBytes`
  (params (Bytes :type "Array of Byte (by ref)") (IPAddress :type String) (Port :type "Integer (by ref)"))
  (`KismetSystemLibrary.PrintString` "Received bytes!")
  (`self.ParseMessage` Bytes))

(fn `GetInfo`
  (`UDPComponent.EmitBytes` (`self.UDP`) (`self.GetInfoArray`))
  (`KismetSystemLibrary.PrintString` "Requested Info")
  (return))

(fn `Ping`
  (`UDPComponent.EmitBytes` (`self.UDP`) (`self.GetPingMessage`))
  (`KismetSystemLibrary.PrintString` "Ping!" true true (struct :`G` 0.66 :`B` 1.0 :`A` 1.0) 1.0)
  (return))

(fn `UserConstructionScript`)