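; Bluetooth LE connection Blueprint for a Ukaton Mission sensor device, with optional auto-connect on BeginPlay and support disabled on Mac.
; Connect scans by service UUIDs, keeps the device accepted by CheckFoundBleDevice, binds read and notification events, then connects.
; A looping timer re-reads device type until the first update, then subscribes to sensor data, configuration and motion calibration.
; Wrapper events forward characteristic read, write, subscribe and unsubscribe calls to the device.
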(event `self.ReceiveBeginPlay`
  (bind _output_get (set `self.bIsBluetoothSupportedForPlatform` (!= (`GameplayStatics.GetPlatformName`) "Mac")))
  (if _output_get
    (bind _returnvalue (`BleUtils.CreateBleManager`))
    (bind _output_get_2 (set `self.BleManager` _returnvalue))
    (if (`BleManagerInterface.IsBleSupported` _output_get_2)
      (`BleManagerInterface.SetBluetoothState` (`self.BleManager`) true)
      (`KismetSystemLibrary.Delay` 0.5)
      (bind _output_get_3 (set `self.bIsBluetoothEnabled` (`BleManagerInterface.IsBluetoothEnabled` (`self.BleManager`))))
      (if _output_get_3
        (`KismetSystemLibrary.PrintString` "enabled ble")
        (if (`self.bAutoConnect`)
          (`self.Connect` (`self.AutoConnectBLEDeviceName`)))
        (else
          (`KismetSystemLibrary.PrintString` "ble not enabled")))
      (else
        (`KismetSystemLibrary.PrintString` "ble not supported")))
    (else
      (`KismetSystemLibrary.PrintString` "bluetooth not supported"))))

(event `self.Connect`
  (params (Name :type String))
  (if (`self.bIsBluetoothSupportedForPlatform`)
    (set `self.bDidFindDevice` false)
    (if (`self.bIsBluetoothEnabled`)
      (`BleManagerInterface.ScanForDevices` (`self.BleManager`) (`self.GetServiceUUIDs`) (delegate `On Device Found`))
      (`KismetSystemLibrary.PrintString` "scanning for devices..."))))

(event `On Device Found`
  (params (Device :type "BleDeviceInterface Interface"))
  (bind (_bledevice _bdidfindbledevice) (`self.Check Found Ble Device` Device (stale `self.Connect` Name)))
  (if _bdidfindbledevice
    (`BleManagerInterface.StopScan` (`self.BleManager`))
    (`KismetSystemLibrary.PrintString` "stopping scan")
    (`BleDeviceInterface.Connect` (`self.BleDevice`) (delegate `On Connect`) (delegate `On Connect Error`))))

(event `OnDeviceTypeUpdated_Event` :!signature `self.OnDeviceTypeUpdated`
  (params (DeviceType :type "EUkatonDeviceType Enum" :default "MOTION_MODULE"))
  (if (not (`self.bDidReceiveFirstResponse`))
    (set `self.bDidReceiveFirstResponse` true)
    (`KismetSystemLibrary.K2_ClearAndInvalidateTimerHandle` (stale `On Connect` _returnvalue))
    (remove `self.OnDeviceTypeUpdated` (delegate `OnDeviceTypeUpdated_Event`))
    (`self.SubscribeToSensorDataCharacteristic`)
    (`self.SubscribeToSensorDataConfigurationsCharacteristic`)
    (`self.SubscribeToMotionCalibrationCharacteristic`)))

(event `On Connect`
  (`KismetSystemLibrary.PrintString` "connected to device")
  (set `self.bDidReceiveFirstResponse` false)
  (bind _returnvalue (`KismetSystemLibrary.K2_SetTimerDelegate` (delegate `CustomEvent`) 0.5 true))
  (add `self.OnDeviceTypeUpdated` (delegate `OnDeviceTypeUpdated_Event`)))

(event `On Connect Error`
  (params (ErrorMessage :type String))
  (`KismetSystemLibrary.PrintString` ErrorMessage true true (struct :`R` 1.0 :`G` 0.0169 :`A` 1.0)))

(event `CustomEvent`
  (`self.ReadDeviceTypeCharacteristic`))

(event `self.Disconnect`
  (if (`BleDeviceInterface.IsConnected` (`self.BleDevice`))
    (`BleDeviceInterface.Disconnect` (`self.BleDevice`) (delegate `On Disconnect`) (delegate `On Disconnect Error`))))

(event `On Disconnect`
  (`KismetSystemLibrary.PrintString` "disconnected")
  (set `self.bDidFindDevice` false))

(event `On Disconnect Error`
  (params (ErrorMessage :type String))
  (`KismetSystemLibrary.PrintString` ErrorMessage))

(event `self.SubscribeToCharacteristic`
  (params (ServiceUUID :type String) (CharacteristicUUID :type String))
  (`BleDeviceInterface.SubscribeToCharacteristic` (`self.BleDevice`) ServiceUUID CharacteristicUUID false))

(event `self.ReadCharacteristic`
  (params (ServiceUUID :type String) (CharacteristicUUID :type String))
  (`BleDeviceInterface.ReadCharacteristic` (`self.BleDevice`) ServiceUUID CharacteristicUUID))

(event `self.WriteCharacteristic`
  (params (ServiceUUID :type String) (CharacteristicUUID :type String) (Data :type "Array of Byte (by ref)"))
  (`BleDeviceInterface.WriteCharacteristic` (`self.BleDevice`) ServiceUUID CharacteristicUUID Data))

(event `self.UnsubscribeFromCharacteristic`
  (params (ServiceUUID :type String) (CharacteristicUUID :type String))
  (`BleDeviceInterface.UnsubscribeFromCharacteristic` (`self.BleDevice`) ServiceUUID CharacteristicUUID))

(fn `BindBleEvents`
  (params (BleDevice :type "BleDeviceInterface Interface"))
  (`BleDeviceInterface.BindToCharacteristicReadEvent` BleDevice (`|CreateDelegate` :!event `OnCharacteristicRead`))
  (`BleDeviceInterface.BindToCharacteristicNotificationEvent` BleDevice (`|CreateDelegate` :!event `OnCharacteristicNotification`))
  (return))

(fn `Check Found Ble Device`
  (params (FoundBleDevice :type "BleDeviceInterface Interface") (Name :type String))
  (returns (BleDevice :type "BleDeviceInterface Interface") (bDidFindBleDevice :type Boolean))
  (if (`KismetStringLibrary.EqualEqual_StrStr` Name Name)
    (if (`self.bDidFindDevice`)
      (if (`KismetStringLibrary.EqualEqual_StrStr` (`BleDeviceInterface.GetDeviceId` (`self.BleDevice`)) (`BleDeviceInterface.GetDeviceId` FoundBleDevice))
        (`KismetSystemLibrary.PrintString` "duplicate device")
        (`self.BindBleEvents` FoundBleDevice)
        (else
          (return null false)))
      (else
        (set `self.bDidFindDevice` true)
        (`KismetSystemLibrary.PrintString` "found device")
        (bind _output_get (set `self.BleDevice` FoundBleDevice))
        (`self.BindBleEvents` _output_get)
        (return _output_get true)))
    (else
      (return null false))))

(fn `UserConstructionScript`)